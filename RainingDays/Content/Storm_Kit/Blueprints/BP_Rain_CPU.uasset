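; CPU rain actor that can follow the player camera at a height offset and drives screen-droplet effects.
; While following, each tick traces upward for cover and checks camera pitch.
; Looking up in the open raises droplet and trail alphas, advances droplet time and fades RainLens volume in by pitch; otherwise the alphas decay and volume drops to near silence.
; The alphas and timer feed MPC_ScreenDropsParameters.
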(event `self.ReceiveTick`
  (params (DeltaSeconds :type "Float (single-precision)"))
  (bind _returnvalue (`GameplayStatics.GetPlayerCameraManager` 0))
  (bind _returnvalue_2 (`GameplayStatics.GetWorldDeltaSeconds`))
  (bind _trailalpha (`self.TrailAlpha`))
  (bind _effectalpha (`self.EffectAlpha`))
  (bind _returnvalue_3 (* _returnvalue_2 0.1))
  (bind _pitch (.pitch (`PlayerCameraManager.GetCameraRotation` _returnvalue)))
  (bind _location (.location (`self.GetTransform` _returnvalue)))
  ;[0 0 0] Makes the rain follow the player
  (if (`self.FollowPlayer`)
    (`self.K2_SetActorLocation` self (`KismetMathLibrary.MakeVector` (.x (`PlayerCameraManager.GetCameraLocation` (`GameplayStatics.GetPlayerCameraManager` 0))) (.y (`PlayerCameraManager.GetCameraLocation` (`GameplayStatics.GetPlayerCameraManager` 0))) (+ (.z (`PlayerCameraManager.GetCameraLocation` (`GameplayStatics.GetPlayerCameraManager` 0))) (`self.Height`))) false false)
    ;[0 0 0] Check if under a roof
    (bind (_outhit _returnvalue_4) (`KismetSystemLibrary.LineTraceSingle` _location (+ _location (0.0 0.0 5000.0)) "TraceTypeQuery1"))
    (if _returnvalue_4
      ;[0 0 0] Scale ScreenDrops effect depending on if player looks up or not
      (set `self.EffectAlpha` (`KismetMathLibrary.FClamp` (- _effectalpha _returnvalue_3)) :!label _label)
      (set `self.TrailAlpha` (`KismetMathLibrary.FClamp` (- _trailalpha (* _returnvalue_2 0.5))))
      (set `self.Volume` 0.01)
      (else
        (`/Engine/EditorBlueprintResources/StandardMacros.CompareFloat` _pitch 40.0
          (:`>`
            (`/Engine/EditorBlueprintResources/StandardMacros.CompareFloat` _pitch 100.0
              (:`>`
                (goto _label))
              (:`<`
                (set `self.EffectAlpha` (`KismetMathLibrary.FClamp` (+ _effectalpha _returnvalue_3)))
                (set `self.TrailAlpha` (`KismetMathLibrary.FClamp` (+ _trailalpha _returnvalue_3)))
                (set `self.Volume` (/ (- (`KismetMathLibrary.FClamp` _pitch 40.0 50.0) 40.0) 10.0))
                (set `self.DropletTime` (+ (`self.DropletTime`) (`GameplayStatics.GetWorldDeltaSeconds`))))))
          (:`<`
            (goto _label)))))
    (`KismetMaterialLibrary.SetScalarParameterValue` "/Game/Storm_Kit/Materials/PostProcess/MPC_ScreenDropsParameters.MPC_ScreenDropsParameters" "Effect_Scale" _effectalpha)
    (`KismetMaterialLibrary.SetScalarParameterValue` "/Game/Storm_Kit/Materials/PostProcess/MPC_ScreenDropsParameters.MPC_ScreenDropsParameters" "TrailsScale" _trailalpha)
    (`KismetMaterialLibrary.SetScalarParameterValue` "/Game/Storm_Kit/Materials/PostProcess/MPC_ScreenDropsParameters.MPC_ScreenDropsParameters" "DropletTime" (`self.DropletTime`))
    (`AudioComponent.SetVolumeMultiplier` (`self.Rain_Lens`) (`self.Volume`))))

(fn `UserConstructionScript`)