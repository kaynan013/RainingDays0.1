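; BP_Clock is a clock Blueprint that displays the current time as text on a TextRender component.
; Every Tick it reads Now and rewrites the text as hour and minute separated by a colon.
; An integer comparison adds a leading zero to minutes below ten, while the hour is left unpadded.
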(event `self.ReceiveTick`
  (params (DeltaSeconds :type "Float (single-precision)"))
  (bind _textrender (`self.TextRender`))
  (bind (_year _month _day _hour _minute) (`KismetMathLibrary.BreakDateTime` (`KismetMathLibrary.Now`)))
  (bind _returnvalue (`KismetStringLibrary.Conv_IntToString` _hour))
  (bind _returnvalue_2 (`KismetStringLibrary.Conv_IntToString` _minute))
  (`/Engine/EditorBlueprintResources/StandardMacros.CompareInt` _minute 10
    (:`>`
      (`TextRenderComponent.K2_SetText` _textrender (`KismetTextLibrary.Conv_StringToText` (`KismetStringLibrary.Concat_StrStr` _returnvalue ":" _returnvalue_2)) :!label _label))
    (:`==`
      (goto _label))
    (:`<`
      (`TextRenderComponent.K2_SetText` _textrender (`KismetTextLibrary.Conv_StringToText` (`KismetStringLibrary.Concat_StrStr` _returnvalue ":" (`KismetStringLibrary.Concat_StrStr` "0" _returnvalue_2)))))))

(fn `UserConstructionScript`)